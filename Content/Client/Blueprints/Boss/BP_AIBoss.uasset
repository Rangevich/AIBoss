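; BP_AIBoss is the boss pawn, driven by an AI controller's Blackboard and shown through an on-screen HP bar widget.
; On BeginPlay it seeds stage and alive keys, while other functions reset the shot cooldown and swap eye materials.
; When a hand's life ends, it clears hand-attack state and enters stage 2 at or below half health.
; Damage broadcasts health updates, and death restarts the level by console command.
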(event `self.ReceivePossessed`
  (params (NewController :type "Controller Object Reference"))
  ; Инициализация босса
  (bind _asaicontroller_boss (cast `/Game/Client/Blueprints/Boss/AI/AIControllerBoss` NewController))
  (set `self.As AIController Boss` _asaicontroller_boss))

(event `self.ReceiveBeginPlay`
  ; Инициализация босса
  (`parent.ReceiveBeginPlay`)
  (set `self.BB_AIBoss` (`AIBlueprintHelperLibrary.GetBlackboard` (`self.As AIController Boss`)))
  (`self.Init`)
  (bind _returnvalue (`|CreateWidget` "/Game/Client/UI/WBP_BossInfo.WBP_BossInfo_C"))
  (`UserWidget.AddToViewport` _returnvalue 0)
  (`/Game/Client/UI/WBP_BossInfo.InitBossHPBar` _returnvalue self))

(event `ResetShootCooldown`
  ; Перезарядка снаряда
  (`BlackboardComponent.SetValueAsBool` (`AIBlueprintHelperLibrary.GetBlackboard` null) (`self.IsShootCooldown`) false))

(event `SwitchMaterialEyes`
  (params (NewMaterial :type "Material Object Reference"))
  ; Изменение материала
  (`PrimitiveComponent.SetMaterial` (`self.Eye1`) 0 NewMaterial)
  (`PrimitiveComponent.SetMaterial` (`self.Eye2`) 0 NewMaterial))

(fn `Die`
  ; Смерть, перезапуск уровня
  (`KismetSystemLibrary.PrintString` "Boss died!" true true (struct :`R` 1.0 :`G` 0.017337 :`A` 1.0))
  (`KismetSystemLibrary.ExecuteConsoleCommand` "RestartLevel" null))

(fn `HandLifeIsOver`
  (`BlackboardComponent.SetValueAsInt` (`AIBlueprintHelperLibrary.GetBlackboard` null) (`self.ProjectileCount`) 0)
  (`BlackboardComponent.SetValueAsBool` (`AIBlueprintHelperLibrary.GetBlackboard` null) (`self.IsHandAttack`) false)
  (if (<= (`self.CurrentHealth`) (/ (`self.MaxHealth`) 2.0))
    (`BlackboardComponent.SetValueAsInt` (`AIBlueprintHelperLibrary.GetBlackboard` null) (`self.Stage`) 2)
    (`KismetSystemLibrary.PrintString` (`KismetStringLibrary.Concat_StrStr` "Стадия - " (`KismetStringLibrary.Conv_IntToString` (`BlackboardComponent.GetValueAsInt` (`AIBlueprintHelperLibrary.GetBlackboard` null) (`self.Stage`)))))))

(fn `Init`
  (`BlackboardComponent.SetValueAsInt` (`self.BB_AIBoss`) (`self.Stage`) (`self.StageNum`))
  (`BlackboardComponent.SetValueAsBool` (`self.BB_AIBoss`) (`self.Alive`) (`self.IsAlive`)))

(fn `TakeDamage`
  (params (Damage :type "Float (double-precision)"))
  (bind _output_get (set `self.CurrentHealth` (- (`self.CurrentHealth`) Damage)))
  (`self.E_HealthUpdated` (`self.CurrentHealth`) (`self.MaxHealth`))
  (if (<= _output_get 0.0)
    (`self.Die`)))

(fn `UserConstructionScript`)