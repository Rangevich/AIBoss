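; BP_Boss is a prototype boss that tracks health, taking damage through TakeDamage and printing the remaining health.
; InitializeBoss runs on BeginPlay to restore health, phase, weak-spot count and body material.
; At zero health, BossDefeated swaps the body material and immediately calls InitializeBoss, so the boss resets at once and the defeat material is overwritten.
; Phase and weak-spot count are only reset here, with no further logic.
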(event `self.ReceiveBeginPlay`
  (`self.InitializeBoss`))

(fn `BossDefeated`
  (`KismetSystemLibrary.PrintString` "Boss defeated")
  (`PrimitiveComponent.SetMaterial` (`self.BossBody`) 0 "/DatasmithContent/Materials/AliasReference.AliasReference")
  (`self.InitializeBoss`))

(fn `InitializeBoss`
  (set `self.CurrentHealth` (`self.MaxHealth`))
  (set `self.Phase` 1)
  (set `self.WeakSpotsHit` 0)
  (`PrimitiveComponent.SetMaterial` (`self.BossBody`) 0 "/Engine/EngineMaterials/WorldGridMaterial.WorldGridMaterial"))

(fn `TakeDamage`
  (bind _currenthealth (`self.CurrentHealth`))
  (set `self.CurrentHealth` (- (`self.CurrentHealth`) (`self.DamageAmount`)))
  (`KismetSystemLibrary.PrintString` (`KismetStringLibrary.Conv_DoubleToString` _currenthealth))
  (if (<= _currenthealth 0.0)
    (`self.BossDefeated`)))

(fn `UserConstructionScript`)