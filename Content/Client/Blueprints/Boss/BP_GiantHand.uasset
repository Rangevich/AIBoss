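; Boss giant hand that follows the player, flips over and slams down, damaging the player once on overlap.
; Tick drives interpolated movement: tracking leads into a rotation Timeline, then a drop to the captured player position, where timer-repeated shockwaves spawn.
; After three shockwaves it spawns weak spots at three random, distinct components tagged WeakPoint.
; Once three are counted destroyed, it destroys itself and notifies BP_AIBoss.
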(event `self.ReceiveBeginPlay`
  (`self.StartTrackingPlayer`))

(event `self.ReceiveTick`
  (params (DeltaSeconds :type "Float (single-precision)"))
  (bind (_returnvalue_x _returnvalue_y _returnvalue_z) (`KismetMathLibrary.BreakVector` (`self.K2_GetActorLocation`)))
  (bind (_returnvalue_x_2 _returnvalue_y_2 _returnvalue_z_2) (`KismetMathLibrary.BreakVector` (`self.K2_GetActorLocation` (`self.TargetPlayer`))))
  (bind (_returnvalue_x_3 _returnvalue_y_3) (`KismetMathLibrary.BreakVector` (`self.K2_GetActorLocation` (`self.TargetPlayer`))))
  (set `self.Delta Seconds` DeltaSeconds)
  ;[0.15 0.103 0.02013 0.5] Создание слабых точек
  (if (and (== (`self.CountSpawnShockwave`) 3) (`self.CanCreateWeekPoint`))
    (`self.CreateWeekSpot`)
    (set `self.CanCreateWeekPoint` false)
    (elif (`self.IsHandAttack`)
      ; Атака кулаком
      (`self.K2_SetActorLocation` (`KismetMathLibrary.VInterpTo` (`self.K2_GetActorLocation`) (`self.TargetLocation`) (`self.Delta Seconds`) (`self.VerticalInterpSpeed`)))
      (if (<= (`KismetMathLibrary.Vector_Distance` (`self.K2_GetActorLocation`) (`self.TargetLocation`)) 30.0)
        (set `self.IsHandAttack` false)
        ;;[0.0448 0.15 0.05769 0.5] Спавн волны
        (`self.SpawnShockwave`)
        (`KismetSystemLibrary.K2_SetTimer` null (`self.Function Name`) 1.0 true))
      (elif (`self.IsTrackPlayer`)
        (if (`self.IsTimelineStarted`)
          _
          (elif (<= (`KismetMathLibrary.Vector_Distance` (`KismetMathLibrary.MakeVector` _returnvalue_x _returnvalue_y) (`KismetMathLibrary.MakeVector` _returnvalue_x_2 _returnvalue_y_2)) (`self.PositionTolerance`))
            ; Переворот кулака
            (set `self.InterpSpeed` (`self.Interp Speed`))
            (set `self.IsTimelineStarted` true)
            (bind (_direction _rotationalpha) (`Timeline|Timeline` :`NewTime` 1.0 :!via `PlayFromStart`)
              (:`Update`
                (`self.K2_SetActorRotation` (`KismetMathLibrary.RLerp` (struct) (struct :`Pitch` -180.0) _rotationalpha))
                (`self.K2_SetActorLocation` (`KismetMathLibrary.VInterpTo` (`KismetMathLibrary.MakeVector` _returnvalue_x _returnvalue_y _returnvalue_z) (`KismetMathLibrary.MakeVector` _returnvalue_x_2 _returnvalue_y_2 (+ _returnvalue_z_2 300.0)) (`self.Delta Seconds`) (`self.InterpSpeed`)) :!label _label))
              (:`Finished`
                (set `self.IsTimelineStarted` false)
                (set `self.IsTrackPlayer` false)
                (set `self.InterpSpeed` (`self.InterpSpeedDefault`))
                (set `self.TargetLocation` (`KismetMathLibrary.MakeVector` _returnvalue_x_3 _returnvalue_y_3 20.0))
                (`self.HandAttack`)))
            (else
              (goto _label))))))))

(event `HandAttack`
  ; Атака рукой
  (set `self.IsDamageWas` false)
  (set `self.IsHandAttack` true))

(event `self.BoxCollision.OnComponentBeginOverlap`
  (params (OverlappedComponent :type "PrimitiveComponent Object Reference") (OtherActor :type "Actor Object Reference") (OtherComp :type "PrimitiveComponent Object Reference") (OtherBodyIndex :type Integer) (bFromSweep :type Boolean) (SweepResult :type "HitResult Structure (by ref)"))
  (bind _asbp_third_person_character (cast `/Game/ThirdPerson/Blueprints/BP_ThirdPersonCharacter` OtherActor))
  (if (not (`self.IsDamageWas`))
    (`/Game/ThirdPerson/Blueprints/BP_ThirdPersonCharacter.TakeDamage` _asbp_third_person_character (`self.DamageHand`))
    (set `self.IsDamageWas` true)
    (`PrimitiveComponent.SetCollisionEnabled` (`self.BoxCollision`) "NoCollision")))

(fn `CountDestroyWeekSpot`
  (set `self.DestroyWeekSpot` (+ (`self.DestroyWeekSpot`) 1))
  (if (== (`self.DestroyWeekSpot`) 3)
    (`self.K2_DestroyActor`)
    (bind _outactors (`GameplayStatics.GetAllActorsOfClass` "/Game/Client/Blueprints/Boss/BP_AIBoss.BP_AIBoss_C"))
    (`/Game/Client/Blueprints/Boss/BP_AIBoss.HandLifeIsOver` (`|GetArrayItem` _outactors))))

(fn `CreateWeekSpot`
  (while (< (`KismetArrayLibrary.Array_Length` (`self.SelectIndexWeekPoint`)) 3)
    ; Рандом индексов точек спавна
    (set `self.SelectIndex` (`KismetMathLibrary.RandomIntegerInRange` 0 (- (`KismetArrayLibrary.Array_Length` (`self.WeakSpotPoints`)) 1)))
    (if (not (`KismetArrayLibrary.Array_Contains` (`self.SelectIndexWeekPoint`) (`self.SelectIndex`)))
      (`KismetArrayLibrary.Array_Add` (`self.SelectIndexWeekPoint`) (`self.SelectIndex`))))
  ;[0.15 0.06789 0.09371 0.5] Создание слабых точек
  (for _array_element (`self.SelectIndexWeekPoint`)
    (`|SpawnActorFromClass` "/Game/Client/Blueprints/Boss/BP_WeakSpot.BP_WeakSpot_C" (`KismetMathLibrary.MakeTransform` (`SceneComponent.K2_GetComponentLocation` (`|GetArrayItem` (`self.WeakSpotPoints`) _array_element))) "Undefined" "MultiplyWithRoot" null null)))

(fn `SpawnShockwave`
  (bind (_returnvalue_x _returnvalue_y _returnvalue_z) (`KismetMathLibrary.BreakVector` (`self.K2_GetActorLocation`)))
  (if (< 2 (`self.CountSpawnShockwave`))
    (`KismetSystemLibrary.K2_ClearTimer` null (`self.Function Name`))
    (else
      (`|SpawnActorFromClass` "/Game/Client/Blueprints/Boss/BP_Shockwave.BP_Shockwave_C" (`KismetMathLibrary.MakeTransform` (`KismetMathLibrary.MakeVector` _returnvalue_x _returnvalue_y (+ _returnvalue_z 0.0))) "Undefined" "MultiplyWithRoot" null null)
      (set `self.CountSpawnShockwave` (+ 1 (`self.CountSpawnShockwave`))))))

(fn `StartTrackingPlayer`
  (set `self.TargetPlayer` (`GameplayStatics.GetPlayerCharacter` 0)))

(fn `UserConstructionScript`
  (for _array_element (`self.K2_GetComponentsByClass` "/Script/Engine.SceneComponent")
    (if (`ActorComponent.ComponentHasTag` _array_element "WeakPoint")
      (`KismetArrayLibrary.Array_Add` (`self.WeakSpotPoints`) _array_element))))