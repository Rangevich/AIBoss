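; Boss laser beam actor that extends a damage capsule until full length, then destroys itself after a short delay.
; Each Tick stretches and shifts the capsule, so growth is frame-rate dependent; on expiry it clears IsLaserCooldown on the tagged Boss's Blackboard.
; Overlap tracks the player and sets a one-shot timer for DamageFunc, which is not defined here; the damage function present is TakePlayerDamage.
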(event `self.ReceiveTick`
  (params (DeltaSeconds :type "Float (single-precision)"))
  (bind _capsulecollisison (`self.CapsuleCollisison`))
  (bind _capsulecollisison_2 (`self.CapsuleCollisison`))
  (bind (_returnvalue_x _returnvalue_y _returnvalue_z) (`KismetMathLibrary.BreakVector` (`SceneComponent.K2_GetComponentScale` (`self.CapsuleCollisison`))))
  (bind (_returnvalue_x_2 _returnvalue_y_2 _returnvalue_z_2) (`KismetMathLibrary.BreakVector` (`SceneComponent.K2_GetComponentScale` _capsulecollisison_2)))
  (if (>= _returnvalue_z 28.0)
    (`KismetSystemLibrary.Delay` 0.5)
    (`self.K2_DestroyActor`)
    (bind _outactors (`GameplayStatics.GetAllActorsWithTag` "Boss"))
    (`BlackboardComponent.SetValueAsBool` (`AIBlueprintHelperLibrary.GetBlackboard` (`|GetArrayItem` _outactors)) (`self.IsLaserCooldown`) false)
    (else
      (`SceneComponent.SetWorldScale3D` _capsulecollisison_2 (`KismetMathLibrary.MakeVector` _returnvalue_x_2 _returnvalue_y_2 (+ _returnvalue_z_2 2.0)))
      (`SceneComponent.K2_SetRelativeLocation` _capsulecollisison (+ (0.0 -90.0 0.0) (`SceneComponent.RelativeLocation` _capsulecollisison)) false false))))

(event `self.CapsuleCollisison.OnComponentBeginOverlap`
  (params (OverlappedComponent :type "PrimitiveComponent Object Reference") (OtherActor :type "Actor Object Reference") (OtherComp :type "PrimitiveComponent Object Reference") (OtherBodyIndex :type Integer) (bFromSweep :type Boolean) (SweepResult :type "HitResult Structure (by ref)"))
  (bind _asbp_third_person_character (cast `/Game/ThirdPerson/Blueprints/BP_ThirdPersonCharacter` OtherActor))
  (set `self.OverlappedPlayer` _asbp_third_person_character)
  (`KismetSystemLibrary.K2_SetTimer` null (`self.DamageFunc`) 0.1))

(event `self.CapsuleCollisison.OnComponentEndOverlap`
  (params (OverlappedComponent :type "PrimitiveComponent Object Reference") (OtherActor :type "Actor Object Reference") (OtherComp :type "PrimitiveComponent Object Reference") (OtherBodyIndex :type Integer))
  (cast `/Game/ThirdPerson/Blueprints/BP_ThirdPersonCharacter` OtherActor)
  (set `self.OverlappedPlayer` null))

(fn `TakePlayerDamage`
  (`/Engine/EditorBlueprintResources/StandardMacros.IsValid` (`self.OverlappedPlayer`)
    (:`Is Valid`
      (`/Game/ThirdPerson/Blueprints/BP_ThirdPersonCharacter.TakeDamage` (`self.OverlappedPlayer`) 10.0))))

(fn `UserConstructionScript`)