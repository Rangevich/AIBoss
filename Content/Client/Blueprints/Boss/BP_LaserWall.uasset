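; BP_LaserWall is a boss hazard with left and right collision boxes meant to damage an overlapping third-person player over time.
; Either box stores the player on begin overlap and starts a looping 0.1-second timer; end overlap clears the reference but not the timer.
; The timer targets "TakePlayerDamageF", while the function shown is TakePlayerDamage, which applies fixed damage to the stored player if valid.
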(event `self.BoxCollisionL.OnComponentBeginOverlap`
  (params (OverlappedComponent :type "PrimitiveComponent Object Reference") (OtherActor :type "Actor Object Reference") (OtherComp :type "PrimitiveComponent Object Reference") (OtherBodyIndex :type Integer) (bFromSweep :type Boolean) (SweepResult :type "HitResult Structure (by ref)"))
  ; Получение урона от левой стены
  (bind _asbp_third_person_character (cast `/Game/ThirdPerson/Blueprints/BP_ThirdPersonCharacter` OtherActor))
  (set `self.OverlappedPlayer` _asbp_third_person_character)
  (`KismetSystemLibrary.K2_SetTimer` null (`self.TakePlayerDamageF`) 0.1 true))

(event `self.BoxCollisionL.OnComponentEndOverlap`
  (params (OverlappedComponent :type "PrimitiveComponent Object Reference") (OtherActor :type "Actor Object Reference") (OtherComp :type "PrimitiveComponent Object Reference") (OtherBodyIndex :type Integer))
  ; Получение урона от левой стены
  (cast `/Game/ThirdPerson/Blueprints/BP_ThirdPersonCharacter` OtherActor)
  (set `self.OverlappedPlayer` null))

(event `self.BoxCollisionR.OnComponentBeginOverlap`
  (params (OverlappedComponent :type "PrimitiveComponent Object Reference") (OtherActor :type "Actor Object Reference") (OtherComp :type "PrimitiveComponent Object Reference") (OtherBodyIndex :type Integer) (bFromSweep :type Boolean) (SweepResult :type "HitResult Structure (by ref)"))
  ; Получение урона от правой стены
  (bind _asbp_third_person_character (cast `/Game/ThirdPerson/Blueprints/BP_ThirdPersonCharacter` OtherActor))
  (set `self.OverlappedPlayer` _asbp_third_person_character)
  (`KismetSystemLibrary.K2_SetTimer` null (`self.TakePlayerDamageF`) 0.1 true))

(event `self.BoxCollisionR.OnComponentEndOverlap`
  (params (OverlappedComponent :type "PrimitiveComponent Object Reference") (OtherActor :type "Actor Object Reference") (OtherComp :type "PrimitiveComponent Object Reference") (OtherBodyIndex :type Integer))
  ; Получение урона от правой стены
  (cast `/Game/ThirdPerson/Blueprints/BP_ThirdPersonCharacter` OtherActor)
  (set `self.OverlappedPlayer` null))

(fn `TakePlayerDamage`
  (`/Engine/EditorBlueprintResources/StandardMacros.IsValid` (`self.OverlappedPlayer`)
    (:`Is Valid`
      (`/Game/ThirdPerson/Blueprints/BP_ThirdPersonCharacter.TakeDamage` (`self.OverlappedPlayer`) 5.0))))

(fn `UserConstructionScript`)