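; BP_PlayerProjectile is the player's projectile that damages the AI boss and its weak spots.
; It shrinks its actor scale on BeginPlay.
; Its Sphere overlap ignores the third-person character, then casts the other actor to the boss or a weak spot, applies PlayerProjectileDamage through TakeDamage and destroys itself.
; Other overlapped actors leave it intact, and movement is not handled in the graph.
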(event `self.ReceiveBeginPlay`
  (`self.SetActorScale3D` (0.3 0.3 0.3)))

(event `self.Sphere.OnComponentBeginOverlap`
  (params (OverlappedComponent :type "PrimitiveComponent Object Reference") (OtherActor :type "Actor Object Reference") (OtherComp :type "PrimitiveComponent Object Reference") (OtherBodyIndex :type Integer) (bFromSweep :type Boolean) (SweepResult :type "HitResult Structure (by ref)"))
  (cast `/Game/ThirdPerson/Blueprints/BP_ThirdPersonCharacter` OtherActor
    (:`CastFailed`
      ; Попадание в босса
      (bind _asbp_aiboss (cast `/Game/Client/Blueprints/Boss/BP_AIBoss` OtherActor)
        (:`then`
          (`/Game/Client/Blueprints/Boss/BP_AIBoss.TakeDamage` _asbp_aiboss (`self.PlayerProjectileDamage`))
          (`self.K2_DestroyActor`))
        (:`CastFailed`
          ;[0.15 0.1318 0.0327 0.5] Попадание в слабую точку
          (bind _asbp_weak_spot (cast `/Game/Client/Blueprints/Boss/BP_WeakSpot` OtherActor))
          (`/Game/Client/Blueprints/Boss/BP_WeakSpot.TakeDamage` _asbp_weak_spot (`self.PlayerProjectileDamage`))
          (`self.K2_DestroyActor`))))))

(fn `UserConstructionScript`)