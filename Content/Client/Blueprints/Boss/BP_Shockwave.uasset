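; BP_Shockwave is a boss shockwave actor that damages player characters it touches.
; On BeginPlay a timeline drives the uniform world scale of the circle component, and the actor destroys itself when the timeline finishes.
; Overlapping a BP_ThirdPersonCharacter calls its TakeDamage with DamageCircle.
; A single flag limits each wave to one hit in total, so only the first character touched is damaged.
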(event `self.ReceiveBeginPlay`
  (bind (_direction _newtrack_1) (`Timeline|Timeline`)
    (:`Update`
      (`SceneComponent.SetWorldScale3D` (`self.Сircle`) (`KismetMathLibrary.MakeVector` _newtrack_1 _newtrack_1 _newtrack_1)))
    (:`Finished`
      (`self.K2_DestroyActor`))))

(event `self.Сircle.OnComponentBeginOverlap`
  (params (OverlappedComponent :type "PrimitiveComponent Object Reference") (OtherActor :type "Actor Object Reference") (OtherComp :type "PrimitiveComponent Object Reference") (OtherBodyIndex :type Integer) (bFromSweep :type Boolean) (SweepResult :type "HitResult Structure (by ref)"))
  (bind _asbp_third_person_character (cast `/Game/ThirdPerson/Blueprints/BP_ThirdPersonCharacter` OtherActor))
  (if (not (`self.IsDamageWas`))
    (`/Game/ThirdPerson/Blueprints/BP_ThirdPersonCharacter.TakeDamage` _asbp_third_person_character (`self.DamageCircle`))
    (set `self.IsDamageWas` true)))

(fn `UserConstructionScript`)