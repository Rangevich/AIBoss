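; BP_WeakSpot is a destructible boss weak spot with its own health and a sphere collision trigger.
; TakeDamage lowers its health and forwards five times the damage to BP_AIBoss; at zero health it destroys itself and notifies BP_GiantHand's destroyed-spot counter.
; Player projectile overlaps call TakeDamage with zero damage.
; Both boss actors are found through GetActorOfClass rather than stored references.
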(event `self.SphereCollision.OnComponentBeginOverlap`
  (params (OverlappedComponent :type "PrimitiveComponent Object Reference") (OtherActor :type "Actor Object Reference") (OtherComp :type "PrimitiveComponent Object Reference") (OtherBodyIndex :type Integer) (bFromSweep :type Boolean) (SweepResult :type "HitResult Structure (by ref)"))
  (cast `/Game/Client/Blueprints/Boss/BP_PlayerProjectile` OtherActor)
  (`self.TakeDamage` 0.0))

(fn `TakeDamage`
  (params (Damage :type "Float (double-precision)"))
  (set `self.Damage` Damage)
  (set `self.CurrentHealth` (- (`self.CurrentHealth`) (`self.Damage`)))
  (bind _returnvalue (`GameplayStatics.GetActorOfClass` "/Game/Client/Blueprints/Boss/BP_AIBoss.BP_AIBoss_C"))
  (`/Game/Client/Blueprints/Boss/BP_AIBoss.TakeDamage` _returnvalue (* (`self.Damage`) 5.0))
  (if (<= (`self.CurrentHealth`) 0.0)
    (`self.K2_DestroyActor`)
    (bind _returnvalue_2 (`GameplayStatics.GetActorOfClass` "/Game/Client/Blueprints/Boss/BP_GiantHand.BP_GiantHand_C"))
    (`/Game/Client/Blueprints/Boss/BP_GiantHand.CountDestroyWeekSpot` _returnvalue_2)))

(fn `UserConstructionScript`)